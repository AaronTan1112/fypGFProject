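; BP_Enemy1_Melee is a melee enemy Blueprint that supplies a swipe attack and its own ideal attack and defend ranges.
; Attack plays the swipe montage sped up and calls OnAttackEnd when it completes or is interrupted.
; A montage notify triggers a short forward sphere trace against pawns, with debug drawing, and sends a damage struct to the hit actor through a TakeDamage message.
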(event EventBeginPlay
  (|CallParentFunction))

(event EventAttack
  (bind _returnvalue (Transformation|GetActorLocation))
  (bind _notifyname (Animation|Montage|PlayMontage (Variables|Character|GetMesh) "/Game/AI/NewEnemy1_2/newEnemy1/Anim/E1/T1_SwipeAtk_Montage.T1_SwipeAtk_Montage" 1.5)
    (:OnCompleted
      (Default|CallOnAttackEnd :!label _label))
    (:OnInterrupted
      (goto _label))
    (:OnNotifyBegin
      (switch name _notifyname
        (:Slash
          (bind _outhit (Collision|SphereTraceForObjects _returnvalue (+ _returnvalue (* (Transformation|GetActorForwardVector) 2e+02)) 2e+01 (Utilities|Array|MakeArray "ObjectTypeQuery3") false 0 "ForDuration"))
          (if true
            (Class|BPIDamagable|TakeDamage(Message) (.HitActor (Collision|BreakHitResult _outhit)) (Utilities|Struct|MakeS_DamageInfo 25.0 "NewEnumerator1"))))))))

(fn ConstructionScript
  (|CallParentFunction))

(fn GetIdealRange
  (return 1.2e+02 5e+02))