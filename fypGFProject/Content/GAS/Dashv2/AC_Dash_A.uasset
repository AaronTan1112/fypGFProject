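; Actor component that gives the third-person character a teleport-style dash with Niagara effects.
; BeginPlay caches the owning BP_ThirdPersonCharacter.
; DashStart teleports it without sweep to the character's TpLocation, spawning the same effect at origin and destination.
; A disconnected DashV2 branch holds a distance-based dash along velocity or forward vector, chosen by LockDash, with optional sweep and separate effects.
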(event Custom|Dash%20Start
  (bind _as_bp_third_person_character (Variables|Default|GetAs%20BP%20Third%20Person%20Character))
  (bind _tplocation (Variables|/Game/ThirdPerson/Blueprints/BP_ThirdPersonCharacter.BP_ThirdPersonCharacter_C|GetTpLocation _as_bp_third_person_character))
  (bind _rootcomponent (Variables|/Script/Engine.Actor|GetRootComponent _as_bp_third_person_character))
  (bind _returnvalue (Transformation|GetWorldTransform _rootcomponent))
  (Niagara|SpawnSystematLocation "/Game/GAS/Dashv2/MDashVFX_NS.MDashVFX_NS" (.location _returnvalue) (.rotation _returnvalue))
  (Transformation|SetWorldLocation _rootcomponent _tplocation false true)
  (Niagara|SpawnSystematLocation "/Game/GAS/Dashv2/MDashVFX_NS.MDashVFX_NS" _tplocation (Transformation|GetActorRotation _as_bp_third_person_character)))

(event EventBeginPlay
  (Utilities|FlowControl|Sequence
    (:then_0
      (bind _asbp_third_person_character (Utilities|Casting|CastToBP_ThirdPersonCharacter (Components|GetOwner)))
      (Variables|Default|SetAs%20BP%20Third%20Person%20Character _asbp_third_person_character))))

(event EventTick
  (params (DeltaSeconds :type Float%20%28single-precision%29)))