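; Ranged enemy child Blueprint that attacks by casting projectiles and supplies its own movement speeds and ideal combat range.
; Attack plays a spell-cast montage whose notifies spawn a projectile at the target or halt movement; completion or interruption restores walking and ends the attack.
; The enemy binds each projectile's hit event and applies damage to Player- or EnemyAI-tagged actors.
; An older attack and a health-based montage stop remain disconnected.
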(event Custom|OnActorHit_Event
  (params (SelfActor :type Actor%20Object%20Reference) (OtherActor :type Actor%20Object%20Reference) (NormalImpulse :type Vector) (Hit :type Hit%20Result%20Structure%20%28by%20ref%29))
  (if (or (Actor|ActorHasTag OtherActor "Player") (Actor|ActorHasTag OtherActor "EnemyAI"))
    (Class|BPIDamagable|TakeDamage(Message) OtherActor (Utilities|Struct|MakeS_DamageInfo 3e+01 "NewEnumerator2") self)))

(event Custom|CustomEvent_1
  (params (SelfActor :type Actor%20Object%20Reference) (OtherActor :type Actor%20Object%20Reference) (NormalImpulse :type Vector) (Hit :type Hit%20Result%20Structure%20%28by%20ref%29))
  ;[1 1 1] Old Event Attack
  (if (or (Actor|ActorHasTag OtherActor "Player") (Actor|ActorHasTag OtherActor "EnemyAI"))
    (Class|BPIDamagable|TakeDamage(Message) OtherActor (Utilities|Struct|MakeS_DamageInfo 2e+01 "NewEnumerator2") self)))

(event EventBeginPlay
  (|CallParentFunction))

(event EventAttack
  (params (AttackTarget :type Actor%20Object%20Reference))
  (|CallParentFunction AttackTarget)
  (bind _notifyname (Animation|Montage|PlayMontage (Variables|Character|GetMesh) "/Game/Characters/Enemy/melee/enemy02_SpellCast_Montage.enemy02_SpellCast_Montage" 2.5)
    (:then
      (Variables|/Game/AI/NewEnemy1_2/DamageSystem/BPC_DamageSystem.BPC_DamageSystem_C|SetIsInterruptable (Variables|Default|GetBPC_DamageSystem) true))
    (:OnCompleted
      (Pawn|Components|CharacterMovement|SetMovementMode (Variables|Character|GetCharacterMovement) "MOVE_Walking" 0 :!label _label)
      (CallFunction|AttackEnd AttackTarget)
      (Variables|/Game/AI/NewEnemy1_2/DamageSystem/BPC_DamageSystem.BPC_DamageSystem_C|SetIsInterruptable (Variables|Default|GetBPC_DamageSystem) true)
      (Variables|Default|SetAttacking false))
    (:OnInterrupted
      (goto _label))
    (:OnNotifyBegin
      (switch name _notifyname
        (:Fire
          (bind _returnvalue (Game|SpawnActorfromClass "/Game/AI/NewEnemy1_2/newEnemy1/BP_ProjectileRangedEnemy1.BP_ProjectileRangedEnemy1_C" (Transformation|GetActorTransform) "Undefined" self 1.5e+03 0.0 AttackTarget false 0))
          (Collision|AssignOnActorHit _returnvalue (delegate Custom|OnActorHit_Event)))
        (:Halt
          (Utilities|FlowControl|Delay 0.2)
          (Pawn|Components|CharacterMovement|DisableMovement (Variables|Character|GetCharacterMovement)))))))

(fn ConstructionScript
  (|CallParentFunction))

(fn SetMovementSpeed
  (params (Speed :type E_MovementSpeed%20Enum :default "NewEnumerator2"))
  (Variables|/Script/Engine.CharacterMovementComponent|SetMaxWalkSpeed (Variables|Character|GetCharacterMovement) (Utilities|Select :Index Speed :NewEnumerator2 0.0 :NewEnumerator0 1e+02 :NewEnumerator1 4e+02 :NewEnumerator3 1e+02 :NewEnumerator4 5e+02))
  (return 0.0))

(fn GetIdealRange
  (return 6e+02 6e+02))