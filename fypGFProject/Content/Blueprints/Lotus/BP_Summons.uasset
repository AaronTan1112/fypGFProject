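; BP_Summons is a summon actor that floats at the player's position, turned to the player's forward direction.
; On BeginPlay it rises to an initial height, then loops MoveComponentTo on its root, bobbing up and down by random amounts over random durations.
; Each eased move targets the player's X and Y, with Z offset from the root's current height.
; The loop continues while the Summon flag is true.
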(event EventBeginPlay
  (bind _returnvalue (Math|Random|RandomFloatinRange 0.5 1.0))
  (bind _returnvalue_2 (Math|Random|RandomFloatinRange 15.0 2e+01))
  (bind _returnvalue_3 (Game|GetPlayerCharacter 0))
  (bind _returnvalue_4 (Game|GetPlayerCharacter 0))
  (bind _defaultsceneroot (Variables|Default|GetDefaultSceneRoot))
  (bind _defaultsceneroot_2 (Variables|Default|GetDefaultSceneRoot))
  (bind _summon (Variables|Default|GetSummon))
  (bind _returnvalue_5 (Transformation|GetWorldLocation _defaultsceneroot))
  (bind _returnvalue_6 (Transformation|GetActorForwardVector _returnvalue_3))
  (bind _returnvalue_7 (Transformation|GetActorLocation _returnvalue_4))
  (bind _returnvalue_8 (Math|Rotator|MakeRotfromX _returnvalue_6))
  (Utilities|FlowControl|DelayUntilNextTick)
  (Components|MoveComponentTo _defaultsceneroot_2 (Math|Vector|MakeVector (.x _returnvalue_7) (.y _returnvalue_7) (.z (+ (Transformation|GetWorldLocation _defaultsceneroot_2) 5e+01))) _returnvalue_8 true true 0.5 false)
  (Components|MoveComponentTo _defaultsceneroot (Math|Vector|MakeVector (.x _returnvalue_7) (.y _returnvalue_7) (.z (+ _returnvalue_2 _returnvalue_5))) _returnvalue_8 true true _returnvalue false :!label _label)
  (if _summon
    (Components|MoveComponentTo _defaultsceneroot (Math|Vector|MakeVector (.x _returnvalue_7) (.y _returnvalue_7) (.z (- _returnvalue_5 _returnvalue_2))) _returnvalue_8 true true _returnvalue false)
    (if _summon
      (goto _label))))

(event EventTick
  (params (DeltaSeconds :type Float%20%28single-precision%29)))

(fn ConstructionScript)