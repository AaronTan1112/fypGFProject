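; TargetLock is an indicator actor that marks the player's current hit actor, likely as a lock-on marker.
; It caches the BP_ThirdPersonCharacter on BeginPlay and polls its HitActor every Tick.
; With a valid target, it shows itself just above the target's origin, offset by the colliding bounds' half-height, copying rotation and scale.
; Without a target, it hides itself.
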(event EventTick
  (params (DeltaSeconds :type Float%20%28single-precision%29))
  (bind _playerref (Variables|Default|GetPlayerRef))
  (bind _hitactor (Variables|/Game/ThirdPerson/Blueprints/BP_ThirdPersonCharacter.BP_ThirdPersonCharacter_C|GethitActor _playerref))
  (bind _returnvalue (Transformation|GetActorTransform _hitactor))
  (Utilities|IsValid _hitactor
    (:Is%20Valid
      (bind _boxextent (Collision|GetActorArrayBounds (Utilities|Array|MakeArray _hitactor) true))
      (Transformation|SetActorTransform (Math|Transform|MakeTransform (+ (.location _returnvalue) (Math|Vector|MakeVector 0.0 0.0 (+ (.z _boxextent) 1.0))) (.rotation _returnvalue) (.scale _returnvalue)))
      (Rendering|SetActorHiddenInGame false))
    (:Is%20Not%20Valid
      (Rendering|SetActorHiddenInGame true))))

(event EventBeginPlay
  (bind _asbp_third_person_character (Utilities|Casting|CastToBP_ThirdPersonCharacter (Game|GetPlayerCharacter 0)))
  (Variables|Default|SetPlayerRef _asbp_third_person_character))

(fn ConstructionScript)