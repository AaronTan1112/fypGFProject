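; BP_NPCInteractable is an NPC that the player can talk to, stepping through dialogue lines.
; A sphere overlap toggles a prompt widget for actors tagged Player.
; Each externally triggered Talk call shows the next line in W_Message, hiding the HUD, disabling movement and setting DisableKeys.
; After the last line it restores these, then resets dialogue following a short cooldown and re-shows the prompt if still overlapped.
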(event OnComponentBeginOverlap(Sphere)
  (params (OverlappedComponent :type Primitive%20Component%20Object%20Reference) (OtherActor :type Actor%20Object%20Reference) (OtherComp :type Primitive%20Component%20Object%20Reference) (OtherBodyIndex :type Integer) (bFromSweep :type Boolean) (SweepResult :type Hit%20Result%20Structure%20%28by%20ref%29))
  (if (and (Actor|ActorHasTag OtherActor "Player") (not (Variables|Default|GetCooldown)))
    (Variables|Default|SetOverlap true)
    (Rendering|SetVisibility (Variables|Default|GetWidget) true false)))

(event OnComponentEndOverlap(Sphere)
  (params (OverlappedComponent :type Primitive%20Component%20Object%20Reference) (OtherActor :type Actor%20Object%20Reference) (OtherComp :type Primitive%20Component%20Object%20Reference) (OtherBodyIndex :type Integer))
  (if (Actor|ActorHasTag OtherActor "Player")
    (Variables|Default|SetOverlap false)
    (Rendering|SetVisibility (Variables|Default|GetWidget) false false)))

(event EventBeginPlay
  (Rendering|SetVisibility (Variables|Default|GetWidget) false false)
  (bind _asbp_third_person_character (Utilities|Casting|CastToBP_ThirdPersonCharacter (Game|Player|GetPlayerPawn 0)))
  (Variables|Default|SetAs%20BP%20Third%20Person%20Character _asbp_third_person_character)
  (Variables|Default|SetdisableKeys false))

(event EventTalk
  (bind _as_bp_third_person_character (Variables|Default|GetAs%20BP%20Third%20Person%20Character))
  (bind _widget (Variables|Default|GetWidget))
  (Widget|SetVisibility (Variables|/Game/ThirdPerson/Blueprints/BP_ThirdPersonCharacter.BP_ThirdPersonCharacter_C|GetHudRef _as_bp_third_person_character) "Hidden")
  (Variables|Default|SetdisableKeys true)
  (Pawn|Components|CharacterMovement|DisableMovement (Variables|/Script/Engine.Character|GetCharacterMovement _as_bp_third_person_character))
  (Math|Integer|IncrementInt (Variables|Default|GetTalkIndex)
    (:%20%20
      (if (< (Variables|Default|GetTalkIndex) (Utilities|Array|Length (Variables|Default|GetDialogue)))
        (Variables|Default|GetUI
          (:then
            _)
          (:else
            (bind _returnvalue (UserInterface|CreateWidget "/Game/GAS/InteractEnv/W_Message.W_Message_C" (Game|GetPlayerController 0)))
            (bind _output_get (Variables|Default|SetUI _returnvalue))
            (UserInterface|Viewport|AddtoViewport _output_get 0)))
        (Rendering|Components|TextRender|SetText (Variables|/Game/GAS/InteractEnv/W_Message.W_Message_C|GetMessageBlock (Variables|Default|GetUI)) (Utilities|Text|ToText(String) (Utilities|Array|Get(acopy) (Variables|Default|GetDialogue) (Variables|Default|GetTalkIndex))))
        (else
          (Widget|SetVisibility (Variables|/Game/ThirdPerson/Blueprints/BP_ThirdPersonCharacter.BP_ThirdPersonCharacter_C|GetHudRef (Variables|Default|GetAs%20BP%20Third%20Person%20Character)) "Visible")
          (Widget|RemovefromParent (Variables|Default|GetUI))
          (Rendering|SetVisibility (Variables|Default|GetWidget) false false)
          (Variables|Default|SetCooldown true)
          (Pawn|Components|CharacterMovement|SetMovementMode (Variables|/Script/Engine.Character|GetCharacterMovement (Variables|Default|GetAs%20BP%20Third%20Person%20Character)) "MOVE_Walking" 0)
          (Variables|Default|SetdisableKeys false)
          (Utilities|FlowControl|Delay 3.0)
          (Variables|Default|SetCooldown false)
          (Variables|Default|SetTalkIndex -1)
          (Variables|Default|SetUI 0)
          (if (Variables|Default|GetOverlap)
            (Rendering|SetVisibility _widget true false)
            (else
              (Rendering|SetVisibility _widget false false))))))))

(fn ConstructionScript)