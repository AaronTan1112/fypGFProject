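; BP_Interactable is an interactable pickup item whose mesh is set from a StaticMesh variable in the construction script.
; The PickUpItem event prints a debug message, waits a tick, then destroys the actor.
; AddToInventory returns the item's name when the AddToInv flag is set.
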(event EventPickUpItem
  (Development|PrintString "Item Picked" true true "(R=0.000000,G=0.660000,B=1.000000,A=1.000000)" 12.0 "")
  (Utilities|FlowControl|DelayUntilNextTick)
  (Actor|DestroyActor))

(fn ConstructionScript
  (Components|StaticMesh|SetStaticMesh (Variables|Default|GetModel) (Variables|Default|GetStaticMesh)))

(fn AddtoInventory
  (if (Variables|Default|GetAddToInv?)
    (return (Variables|Default|GetItemName))))