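; Boss enemy, built on a parent enemy class, with projectile basic and barrage attacks, a lightning AOE strike, self-heal and teleport.
; Montage notifies fire projectiles and halt movement, while damage and attack components handle health, interruptibility, strikes and healing.
; Teleport is a hidden high-speed AI flight with dash trail effects and pawn collision ignored.
; Tick opens the Title level after a delay once health reaches zero.
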(event Custom|Teleport
  (params (Location :type Vector))
  (bind _charactermovement (Variables|Character|GetCharacterMovement))
  ;[1 1 1] Teleport Start & End
  (if (not (Variables|Default|GetIsTeleporting))
    (Variables|Default|SetIsTeleporting true)
    (Pawn|Components|CharacterMovement|SetMovementMode _charactermovement "MOVE_Flying" 0)
    (Variables|/Script/Engine.CharacterMovementComponent|SetMaxFlySpeed _charactermovement 5e+03)
    (Variables|/Script/Engine.CharacterMovementComponent|SetMaxAcceleration _charactermovement 99999.0)
    (Rendering|SetVisibility (Variables|Character|GetMesh) false true)
    (Collision|SetCollisionResponsetoChannel (Variables|Default|GetCapsuleComponent) "ECC_Pawn" "ECR_Ignore")
    (bind _returnvalue (Niagara|SpawnSystematLocation "/Game/KTP_Effect/Particles/Fly/VFXINUSE/sdashtrail.sdashtrail" (Transformation|GetActorLocation) (Transformation|GetActorRotation)))
    (Variables|Default|SetTeleportBodyEffect _returnvalue)
    (bind _returnvalue_2 (Niagara|SpawnSystemAttached "/Game/KTP_Effect/Particles/Fly/VFXINUSE/edashtrail.edashtrail" (Variables|Character|GetMesh) "Bip001-Pelvis" "0, 0, 0" "0, 0, 0" "KeepRelativeOffset" false))
    (Variables|Default|SetTelepotTrailEffect _returnvalue_2)
    (Animation|StopAnimMontage 0)
    (AI|AIMoveTo self Location 0 15.0 false
      (:OnSuccess
        _)
      (:OnFail
        _))
    (CallFunction|TeleportEnd)
    (else
      (Utilities|FlowControl|DelayUntilNextTick)
      (Default|CallOnTeleportEnd))))

(event Custom|CustomEvent
  (params (SelfActor :type Actor%20Object%20Reference) (OtherActor :type Actor%20Object%20Reference) (NormalImpulse :type Vector) (Hit :type Hit%20Result%20Structure%20%28by%20ref%29))
  ;[1 1 1] Auto Attack
  (if (or (Actor|ActorHasTag OtherActor "Player") (Actor|ActorHasTag OtherActor "EnemyAI"))
    (Class|BPIDamagable|TakeDamage(Message) OtherActor (Utilities|Struct|MakeS_DamageInfo 15.0 "NewEnumerator2") self)))

(event Custom|TeleportEnd
  (bind _charactermovement (Variables|Character|GetCharacterMovement))
  ;[1 1 1] Teleport Start & End
  (Components|Movement|StopMovementImmediately _charactermovement)
  (Pawn|Components|CharacterMovement|SetMovementMode _charactermovement "MOVE_Walking" 0)
  (Variables|/Script/Engine.CharacterMovementComponent|SetMaxAcceleration _charactermovement 1.5e+03)
  (Rendering|SetVisibility (Variables|Character|GetMesh) true true)
  (Collision|SetCollisionResponsetoChannel (Variables|Default|GetCapsuleComponent) "ECC_Pawn" "ECR_Block")
  (Default|CallOnTeleportEnd)
  (Utilities|FlowControl|Delay 0.5)
  (Variables|Default|SetIsTeleporting false)
  (Utilities|FlowControl|Sequence
    (:then_0
      (bind _teleportbodyeffect (Variables|Default|GetTeleportBodyEffect)
        (:then
          (Components|DestroyComponent _teleportbodyeffect))
        (:else)))
    (:then_1
      (bind _telepottraileffect (Variables|Default|GetTelepotTrailEffect)
        (:then
          (Components|DestroyComponent _telepottraileffect))
        (:else)))))

(event Custom|AOEStrike
  (params (Attack%20Target :type Actor%20Object%20Reference))
  ;[1 1 1] AOEStrike
  (|CallParentFunction Attack%20Target)
  (Utilities|FlowControl|Sequence
    (:then_0
      (Pawn|Components|CharacterMovement|DisableMovement (Variables|Character|GetCharacterMovement)))
    (:then_1
      (Animation|Montage|PlayMontage (Variables|Character|GetMesh) "/Game/Characters/Enemy/melee/enemy_AOESpell_Montage.enemy_AOESpell_Montage"
        (:then
          (Variables|/Game/AI/NewEnemy1_2/DamageSystem/BPC_DamageSystem.BPC_DamageSystem_C|SetIsInterruptable (Variables|Default|GetBPC_DamageSystem) false))
        (:OnCompleted
          (Pawn|Components|CharacterMovement|SetMovementMode (Variables|Character|GetCharacterMovement) "MOVE_Walking" 0 :!label _label)
          (CallFunction|AttackEnd Attack%20Target)
          (Variables|/Game/AI/NewEnemy1_2/DamageSystem/BPC_DamageSystem.BPC_DamageSystem_C|SetIsInterruptable (Variables|Default|GetBPC_DamageSystem) false))
        (:OnInterrupted
          (goto _label))))
    (:then_2
      (Utilities|FlowControl|Delay 0.5) ; Add Attack end here to make the aoe more aggro
      (Default|LightningStrike (Variables|Default|GetBPC_Attacks) Attack%20Target 1.0 35.0))))

(event Custom|BarrageAttack
  (params (AttackTarget :type Actor%20Object%20Reference))
  ;[1 1 1] Barrage Attack
  (|CallParentFunction AttackTarget)
  (bind _notifyname (Animation|Montage|PlayMontage (Variables|Character|GetMesh) "/Game/Characters/Enemy/melee/BossBarrageAtk_Montage.BossBarrageAtk_Montage" 1.5)
    (:then
      (Variables|/Game/AI/NewEnemy1_2/DamageSystem/BPC_DamageSystem.BPC_DamageSystem_C|SetIsInterruptable (Variables|Default|GetBPC_DamageSystem) false))
    (:OnCompleted
      (Pawn|Components|CharacterMovement|SetMovementMode (Variables|Character|GetCharacterMovement) "MOVE_Walking" 0 :!label _label)
      (CallFunction|AttackEnd AttackTarget)
      (Variables|/Game/AI/NewEnemy1_2/DamageSystem/BPC_DamageSystem.BPC_DamageSystem_C|SetIsInterruptable (Variables|Default|GetBPC_DamageSystem) false)
      (Variables|Default|SetAttacking false))
    (:OnInterrupted
      (goto _label))
    (:OnNotifyBegin
      (switch name _notifyname
        (:Fire
          (bind _returnvalue (Game|SpawnActorfromClass "/Game/AI/NewEnemy1_2/newEnemy1/BP_ProjectileRangedEnemy1v3.BP_ProjectileRangedEnemy1v3_C" (Math|Transform|MakeTransform (Transformation|GetSocketLocation (Variables|Character|GetMesh) "Bip001-L-Hand") (Math|Rotator|FindLookatRotation (Transformation|GetActorLocation) (+ (Transformation|GetActorLocation AttackTarget) (Math|Vector|MakeVector 0.0 (Math|Random|RandomFloatinRange -4e+02 4e+02) 0.0))) "1.000000,1.000000,1.000000") "Undefined" self 2e+03 0.0 AttackTarget false 0))
          (Collision|AssignOnActorHit _returnvalue (delegate Custom|CustomEvent_1)))
        (:Halt
          (Utilities|FlowControl|Delay 0.2)
          (Pawn|Components|CharacterMovement|DisableMovement (Variables|Character|GetCharacterMovement)))))))

(event Custom|SelfHeal
  (params (AttackTarget :type Actor%20Object%20Reference))
  ;[1 1 1] Self Heal
  (|CallParentFunction AttackTarget)
  (Pawn|Components|CharacterMovement|DisableMovement (Variables|Character|GetCharacterMovement))
  (Animation|Montage|PlayMontage (Variables|Character|GetMesh) "/Game/Characters/Enemy/melee/enemy_Healing_Montage.enemy_Healing_Montage"
    (:then
      (Default|HealTarget (Variables|Default|GetBPC_Attacks) self)
      (Utilities|FlowControl|Delay 3.0)
      (CallFunction|AttackEnd AttackTarget))))

(event Custom|CustomEvent_1
  (params (SelfActor :type Actor%20Object%20Reference) (OtherActor :type Actor%20Object%20Reference) (NormalImpulse :type Vector) (Hit :type Hit%20Result%20Structure%20%28by%20ref%29))
  ;[1 1 1] Barrage Attack
  (if (Actor|ActorHasTag OtherActor "Player")
    (Class|BPIDamagable|TakeDamage(Message) OtherActor (Utilities|Struct|MakeS_DamageInfo 25.0 "NewEnumerator2") self)))

(event Custom|BasicAttack
  (params (AttackTarget :type Actor%20Object%20Reference))
  ;[1 1 1] Auto Attack
  (|CallParentFunction AttackTarget)
  (bind _notifyname (Animation|Montage|PlayMontage (Variables|Character|GetMesh) "/Game/Characters/Enemy/melee/enemyBoss_SpellCastAmp_Montage1.enemyBoss_SpellCastAmp_Montage1" 1.5)
    (:then
      (Variables|/Game/AI/NewEnemy1_2/DamageSystem/BPC_DamageSystem.BPC_DamageSystem_C|SetIsInterruptable (Variables|Default|GetBPC_DamageSystem) false))
    (:OnCompleted
      (Pawn|Components|CharacterMovement|SetMovementMode (Variables|Character|GetCharacterMovement) "MOVE_Walking" 0 :!label _label)
      (CallFunction|AttackEnd AttackTarget)
      (Variables|/Game/AI/NewEnemy1_2/DamageSystem/BPC_DamageSystem.BPC_DamageSystem_C|SetIsInterruptable (Variables|Default|GetBPC_DamageSystem) false)
      (Variables|Default|SetAttacking false))
    (:OnInterrupted
      (goto _label))
    (:OnNotifyBegin
      (switch name _notifyname
        (:Fire
          (bind _returnvalue (Game|SpawnActorfromClass "/Game/AI/NewEnemy1_2/newEnemy1/BP_ProjectileRangedEnemy1v3.BP_ProjectileRangedEnemy1v3_C" (Transformation|GetActorTransform) "Undefined" self 4e+03 0.0 0 false 0))
          (Collision|AssignOnActorHit _returnvalue (delegate Custom|CustomEvent)))
        (:Halt
          (Utilities|FlowControl|Delay 0.2)
          (Pawn|Components|CharacterMovement|DisableMovement (Variables|Character|GetCharacterMovement)))))))

(event EventBeginPlay
  (|CallParentFunction)
  (Variables|/Game/AI/NewEnemy1_2/DamageSystem/BPC_DamageSystem.BPC_DamageSystem_C|SetIsInterruptable (Variables|Default|GetBPC_DamageSystem) true))

(event EventTick
  (params (DeltaSeconds :type Float%20%28single-precision%29))
  (bind _health (CallFunction|GetCurrentHealth))
  (if (<= _health 0.0)
    (Utilities|FlowControl|Delay 5.0)
    (Game|OpenLevel(byObjectReference) "/Game/Game_Level_ActualVer/TitleScreen/Title.Title")))

(event EventAttack
  (params (AttackTarget :type Actor%20Object%20Reference))
  (|CallParentFunction AttackTarget))

(fn ConstructionScript
  (bind _bpc_damagesystem (Variables|Default|GetBPC_DamageSystem))
  (|CallParentFunction)
  (Variables|/Game/AI/NewEnemy1_2/DamageSystem/BPC_DamageSystem.BPC_DamageSystem_C|SetMaxHealth _bpc_damagesystem 2.5e+02)
  (Variables|/Game/AI/NewEnemy1_2/DamageSystem/BPC_DamageSystem.BPC_DamageSystem_C|SetHealth _bpc_damagesystem 2.5e+02))

(fn SetMovementSpeed
  (params (Speed :type E_MovementSpeed%20Enum :default "NewEnumerator2"))
  (bind _output_get (Variables|/Script/Engine.CharacterMovementComponent|SetMaxWalkSpeed (Variables|Character|GetCharacterMovement) (Utilities|Select :Index Speed :NewEnumerator2 0.0 :NewEnumerator0 1e+02 :NewEnumerator1 8e+02 :NewEnumerator3 1e+02 :NewEnumerator4 5e+02)))
  (return _output_get))

(fn GetIdealRange
  (return 1e+03 1.2e+03))