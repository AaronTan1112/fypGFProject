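; AC_Blink is a component that gives the player character a short forward blink.
; BlinkStart spawns a start effect, waits briefly, moves player 0's capsule forward by BlinkDistance, then spawns an end effect at the new location.
; The move sweeps for collision rather than teleporting through obstacles.
; BeginPlay does nothing and the owner cast is unconnected, so the blink always targets player 0 rather than the owner.
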(event Custom|BlinkStart
  (bind _returnvalue (Game|GetPlayerCharacter 0))
  (bind _capsulecomponent (Variables|/Script/Engine.Character|GetCapsuleComponent _returnvalue))
  (bind _returnvalue_2 (Transformation|GetWorldLocation _capsulecomponent))
  (Niagara|SpawnSystematLocation "/Game/RaihanStuff/StartBlink.StartBlink" _returnvalue_2)
  (Utilities|FlowControl|Delay 0.2)
  (Transformation|SetWorldLocation _capsulecomponent (+ _returnvalue_2 (* (Math|Vector|GetForwardVector _capsulecomponent) (Variables|Default|GetBlink%20Distance))) true false)
  (Niagara|SpawnSystematLocation "/Game/RaihanStuff/EndBlink.EndBlink" (Transformation|GetWorldLocation (Variables|/Script/Engine.Character|GetCapsuleComponent (Game|GetPlayerCharacter 0)))))

(event EventBeginPlay
  (Utilities|FlowControl|Sequence))