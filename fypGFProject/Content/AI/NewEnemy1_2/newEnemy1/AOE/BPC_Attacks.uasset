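; Actor component in the enemy AI folder that provides two area-of-effect attack abilities: a lightning strike and a targeted heal.
; LightningStrike spawns a delayed strike actor at the target with the owning pawn as instigator, then damages overlapped actors through a TakeDamage message.
; HealTarget line-traces for a surface, spawns and triggers a timed heal area there, and sends a Heal message only when the intended target overlaps.
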(event Custom|HealTarget
  (params (HealTarget :type Actor%20Object%20Reference))
  (bind _returnvalue (Transformation|GetActorLocation HealTarget))
  (Utilities|IsValid HealTarget
    (:Is%20Valid
      (bind (_outhit _returnvalue_2) (Collision|LineTraceByChannel _returnvalue (* _returnvalue "1.000000,1.000000,-1000.000000") "TraceTypeQuery1" false (Utilities|Array|MakeArray HealTarget) "None"))
      (if _returnvalue_2
        (bind _returnvalue_3 (Game|SpawnActorfromClass "/Game/AI/NewEnemy1_2/newEnemy1/AOE/BP_AOE_Heal.BP_AOE_Heal_C" (Math|Transform|MakeTransform (.Location (Collision|BreakHitResult _outhit)) "0, 0, 0" "1.000000,1.000000,1.000000") "Undefined" 0 1.0 1e+01 false true false 0))
        (EventDispatchers|AssignOnAOEOverlapActor _returnvalue_3 (delegate Custom|OnHealTarget))
        (Default|Trigger _returnvalue_3)))))

(event Custom|LightningStrike
  (params (AttackTarget :type Actor%20Object%20Reference) (DelayBeforeStrike :type Float%20%28single-precision%29) (DamageAmount :type Float%20%28double-precision%29))
  (bind _returnvalue (Components|GetOwner))
  (bind (_aspawn _bsuccess) (Utilities|Casting|CastToPawn _returnvalue))
  (bind _returnvalue_2 (Game|SpawnActorfromClass "/Game/AI/NewEnemy1_2/newEnemy1/AOE/BP_AOE_LightningStrike.BP_AOE_LightningStrike_C" (Math|Transform|MakeTransform (Transformation|GetActorLocation AttackTarget) "0, 0, 0" "1.000000,1.000000,1.000000") "Undefined" 0 DelayBeforeStrike AttackTarget true true false (select _bsuccess _aspawn 0)))
  (EventDispatchers|BindEventtoOnAOEOverlapActor _returnvalue_2 (delegate Custom|DamageEventAOE)))

(event Custom|DamageEventAOE
  (params (Actor :type Actor%20Object%20Reference))
  (Class|BPIDamagable|TakeDamage(Message) Actor (Utilities|Struct|MakeS_DamageInfo (stale Custom|LightningStrike DamageAmount) "NewEnumerator3")))

(event Custom|OnHealTarget
  (params (Actor :type Actor%20Object%20Reference))
  (if (== Actor (stale Custom|HealTarget HealTarget))
    (Class|BPIDamagable|Heal(Message) Actor 1e+01)
    (Development|PrintString "Hello")))

(event EventBeginPlay)

(event EventTick
  (params (DeltaSeconds :type Float%20%28single-precision%29)))