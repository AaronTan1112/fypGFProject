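; BP_Wave is an expanding wave that damages enemies and makes them wet.
; Each tick it widens its Cylinder horizontally at a frame-rate-independent speed, then destroys itself at the size limit.
; On overlap, damageable actors tagged EnemyAI take buff-modified damage credited to the player character.
; Each hit also spawns a BP_Debuff, attaches it to the enemy and calls Wet on it.
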(event EventTick
  (params (DeltaSeconds :type Float%20%28single-precision%29))
  (Utilities|Expand 0.5 2e+01))

(event Collision|EventActorBeginOverlap
  (params (OtherActor :type Actor%20Object%20Reference))
  (bind _returnvalue (Game|GetPlayerCharacter 0))
  (if (and (Utilities|DoesObjectImplementInterface OtherActor "/Game/AI/NewEnemy1_2/DamageSystem/BPI_Damagable.BPI_Damagable_C") (Actor|ActorHasTag OtherActor "EnemyAI"))
    (Utilities|FlowControl|Sequence
      (:then_0
        (bind _buffedamount (Class|BPIDamagable|PlayerBuffModifier(Message) _returnvalue 4e+01))
        (Class|BPIDamagable|TakeDamage(Message) OtherActor (Utilities|Struct|MakeS_DamageInfo _buffedamount "NewEnumerator3" "NewEnumerator4") _returnvalue)
        (bind _returnvalue_2 (Game|SpawnActorfromClass "/Game/Blueprints/Lotus/BP_Debuff.BP_Debuff_C" (Math|Transform|MakeTransform "0, 0, 0") "Undefined" 0 0))
        (Transformation|AttachActorToActor _returnvalue_2 OtherActor "None" "SnapToTarget" "SnapToTarget" "SnapToTarget" true)
        (Default|Wet _returnvalue_2)))))

(fn ConstructionScript)