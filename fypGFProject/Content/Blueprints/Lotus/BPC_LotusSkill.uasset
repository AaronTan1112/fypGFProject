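; Actor component implementing the Lotus character's four skills, each charging mana and starting a cooldown on the player.
; Skills spawn a root, a timed buff with a summon, delayed heal pulses, and a delayed wave whose destruction clears all BP_Debuff actors, healing for each.
; Predicted projectile paths against world geometry place root, heal and wave effects.
; A TargetSkill1 event moves an aimed root preview; several older implementations remain disconnected.
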(event Custom|CastSkill1
  (params (Player :type BP%20Third%20Person%20Character%20Object%20Reference))
  (bind _returnvalue (Game|GetPlayerCharacter 0))
  (bind _skill1cd (Variables|/Game/ThirdPerson/Blueprints/BP_ThirdPersonCharacter.BP_ThirdPersonCharacter_C|GetSkill1CD Player))
  (bind _hitactor (Variables|/Game/ThirdPerson/Blueprints/BP_ThirdPersonCharacter.BP_ThirdPersonCharacter_C|GethitActor Player))
  ;[1 1 1] Skill1
  (Utilities|IsValid _hitactor
    (:Is%20Valid
      (Variables|S1|SetStartPos (Transformation|GetActorLocation _hitactor))
      (Variables|S1|SetLaunchVelo "0.000000,0.000000,-750.000000"))
    (:Is%20Not%20Valid
      (Variables|S1|SetStartPos (+ (Transformation|GetActorLocation _returnvalue) "0.000000,0.000000,50.000000"))
      (Variables|S1|SetLaunchVelo (* (Transformation|GetActorForwardVector _returnvalue) 1000))))
  (bind _outhit (Class|GameplayStatics|BlueprintPredictProjectilePathbyObjectType (Variables|S1|GetStartPos) (Variables|S1|GetLaunchVelo) true 0.0 (Utilities|Array|MakeArray "ObjectTypeQuery1") false 0 "None"))
  (Niagara|SpawnSystematLocation "/Game/GAS/Roots/RootP1VFX_NS.RootP1VFX_NS" (.Location (Collision|BreakHitResult _outhit)) "0, 0, 0" "1.000000,1.000000,1.000000" true true "AutoRelease")
  (Game|SpawnActorfromClass "/Game/Blueprints/Lotus/BP_Root.BP_Root_C" (Math|Transform|MakeTransform (.Location (Collision|BreakHitResult _outhit)) (Math|Rotator|MakeRotfromZ (.Normal (Collision|BreakHitResult _outhit)))) "Undefined" 0 0)
  (Default|ManaChange Player (Variables|Default|GetManaCostS1))
  (bind _timeref (Default|SkillonCD Player _skill1cd 5.0))
  (Utilities|FlowControl|Delay _timeref)
  (Default|SkillonCD Player _skill1cd 0.0))

(event Custom|Skill3
  (params (PlayerRef :type BP%20Third%20Person%20Character%20Object%20Reference))
  (bind _skill3cd (Variables|/Game/ThirdPerson/Blueprints/BP_ThirdPersonCharacter.BP_ThirdPersonCharacter_C|GetSkill3CD PlayerRef))
  (bind _bpc_damagesystem (Variables|/Game/ThirdPerson/Blueprints/BP_ThirdPersonCharacter.BP_ThirdPersonCharacter_C|GetBPC_DamageSystem PlayerRef))
  ;[1 1 1] Skill3
  (bind _outhit (Class|GameplayStatics|BlueprintPredictProjectilePathbyObjectType (Transformation|GetActorLocation (Game|GetPlayerCharacter 0)) "0.000000,0.000000,-750.000000" true 0.0 (Utilities|Array|MakeArray "ObjectTypeQuery1") false 0 "None"))
  (Niagara|SpawnSystematLocation "/Game/GAS/LotusLeaf/LotusLeafVFX_NS.LotusLeafVFX_NS" (.Location (Collision|BreakHitResult _outhit)))
  (Utilities|FlowControl|Sequence
    (:then_0
      (Default|ManaChange PlayerRef (Variables|Default|GetManaCostS3))
      (Utilities|FlowControl|Delay 1.5)
      (bind _buffedamount (Default|PlayerBuffModifier PlayerRef 5.0))
      (Default|Heal _bpc_damagesystem _buffedamount)
      (Utilities|FlowControl|Sequence
        (:then_0
          (goto _label Reset))
        (:then_1
          (Utilities|FlowControl|DoN 5 :!label _label
            (:Exit
              (Utilities|FlowControl|Delay 1.6)
              (bind _buffedamount_2 (Default|PlayerBuffModifier PlayerRef 7.0))
              (Default|Heal _bpc_damagesystem _buffedamount_2)
              (Utilities|FlowControl|Delay 1.5)
              (bind _buffedamount_3 (Default|PlayerBuffModifier PlayerRef 1e+01))
              (Default|Heal _bpc_damagesystem _buffedamount_3))))))
    (:then_1
      (bind _timeref (Default|SkillonCD PlayerRef _skill3cd 5.0))
      (Utilities|FlowControl|Delay _timeref)
      (Default|SkillonCD PlayerRef _skill3cd 5.0))))

(event Custom|CastSkill2
  (params (ThirdPersonBP :type BP%20Third%20Person%20Character%20Object%20Reference))
  (bind _skill2cd (Variables|/Game/ThirdPerson/Blueprints/BP_ThirdPersonCharacter.BP_ThirdPersonCharacter_C|GetSkill2CD ThirdPersonBP))
  (bind _mesh (Variables|/Script/Engine.Character|GetMesh ThirdPersonBP))
  (bind _summonlocation (Variables|/Game/ThirdPerson/Blueprints/BP_ThirdPersonCharacter.BP_ThirdPersonCharacter_C|GetSummonLocation ThirdPersonBP))
  (bind _returnvalue (Transformation|GetWorldTransform _summonlocation))
  ;[1 1 1] Skill2
  (Variables|/Game/ThirdPerson/Blueprints/BP_ThirdPersonCharacter.BP_ThirdPersonCharacter_C|SetIsBuff ThirdPersonBP true)
  (Rendering|Material|SetOverlayMaterial _mesh "/Game/GAS/Lotus4th/meshMat_Inst1.meshMat_Inst1" :!class /Script/Engine.MeshComponent)
  (Game|SpawnActorfromClass "/Game/Blueprints/Lotus/BP_Summons.BP_Summons_C" (Math|Transform|MakeTransform (.location _returnvalue) (.rotation _returnvalue) "0.100000,0.100000,0.100000") "AlwaysSpawn" 0 0)
  (Default|ManaChange ThirdPersonBP (Variables|Default|GetManaCostS2))
  (Utilities|FlowControl|Sequence
    (:then_0
      (bind _timeref (Default|SkillonCD ThirdPersonBP _skill2cd 15.0))
      (Utilities|FlowControl|Delay _timeref)
      (Default|SkillonCD ThirdPersonBP _skill2cd 15.0))
    (:then_1
      (Utilities|FlowControl|Delay 1e+01) ; Buff Duration
      (Variables|/Game/ThirdPerson/Blueprints/BP_ThirdPersonCharacter.BP_ThirdPersonCharacter_C|SetIsBuff ThirdPersonBP false)
      (Rendering|Material|SetOverlayMaterial _mesh "/Game/GAS/Lotus4th/meshMat_Inst.meshMat_Inst" :!class /Script/Engine.MeshComponent))))

(event Custom|Skill4
  (params (PlayerRef :type BP%20Third%20Person%20Character%20Object%20Reference))
  (bind _returnvalue (Game|GetPlayerCharacter 0))
  (bind _skill4cd (Variables|/Game/ThirdPerson/Blueprints/BP_ThirdPersonCharacter.BP_ThirdPersonCharacter_C|GetSkill4CD PlayerRef))
  (bind _outhit (Class|GameplayStatics|BlueprintPredictProjectilePathbyObjectType (+ (Transformation|GetActorLocation _returnvalue) "0.000000,0.000000,50.000000") (* (Transformation|GetActorForwardVector _returnvalue) 1000) true 0.0 (Utilities|Array|MakeArray "ObjectTypeQuery1") false 0 "None"))
  (Niagara|SpawnSystematLocation "/Game/GAS/Lotus4th/lotus4v2VFX_NS.lotus4v2VFX_NS" (.Location (Collision|BreakHitResult _outhit)) "0, 0, 0" "1.000000,1.000000,1.000000" true true "AutoRelease")
  (Utilities|FlowControl|Sequence
    (:then_0
      (Utilities|FlowControl|Delay 3.8)
      (bind _returnvalue_2 (Game|SpawnActorfromClass "/Game/Blueprints/Lotus/BP_Wave.BP_Wave_C" (Math|Transform|MakeTransform (.Location (Collision|BreakHitResult _outhit)) (Math|Rotator|MakeRotfromZ (.Normal (Collision|BreakHitResult _outhit)))) "Undefined" 0 0))
      (Game|AssignOnDestroyed _returnvalue_2 (delegate Custom|OnDestroyed_Event))
      (bind _timeref (Default|SkillonCD PlayerRef _skill4cd 5.0))
      (Utilities|FlowControl|Delay _timeref)
      (Default|SkillonCD PlayerRef _skill4cd 5.0))
    (:then_1
      (Default|ManaChange PlayerRef (Variables|Default|GetManaCostS4))
      (Variables|/Game/AI/NewEnemy1_2/DamageSystem/BPC_DamageSystem.BPC_DamageSystem_C|SetIsInterruptable (Variables|/Game/ThirdPerson/Blueprints/BP_ThirdPersonCharacter.BP_ThirdPersonCharacter_C|GetBPC_DamageSystem PlayerRef) true))))

(event Custom|Skill4Proc
  (params (PlayerRef :type BP%20Third%20Person%20Character%20Object%20Reference))
  (Variables|/Game/AI/NewEnemy1_2/DamageSystem/BPC_DamageSystem.BPC_DamageSystem_C|SetIsInterruptable (Variables|/Game/ThirdPerson/Blueprints/BP_ThirdPersonCharacter.BP_ThirdPersonCharacter_C|GetBPC_DamageSystem PlayerRef) false)
  (bind _outactors (Actor|GetAllActorsOfClass "/Game/Blueprints/Lotus/BP_Debuff.BP_Debuff_C"))
  (for _array_element _outactors
    (Actor|DestroyActor _array_element)
    (Utilities|FlowControl|Delay 0.5)
    (bind _buffedamount (Default|PlayerBuffModifier PlayerRef 1e+01))
    (Default|Heal (Variables|/Game/ThirdPerson/Blueprints/BP_ThirdPersonCharacter.BP_ThirdPersonCharacter_C|GetBPC_DamageSystem PlayerRef) _buffedamount))
  (Variables|/Game/AI/NewEnemy1_2/DamageSystem/BPC_DamageSystem.BPC_DamageSystem_C|SetIsInterruptable (Variables|/Game/ThirdPerson/Blueprints/BP_ThirdPersonCharacter.BP_ThirdPersonCharacter_C|GetBPC_DamageSystem PlayerRef) true))

(event Custom|OnDestroyed_Event
  (params (DestroyedActor :type Actor%20Object%20Reference))
  (CallFunction|Skill4Proc (stale Custom|Skill4 PlayerRef)))

(event Custom|TargetSkill1
  (bind _returnvalue (Game|GetPlayerCharacter 0))
  (bind _outhit (Class|GameplayStatics|BlueprintPredictProjectilePathbyTraceChannel (+ (Transformation|GetActorLocation _returnvalue) "0.000000,0.000000,50.000000") (* (+ (Math|Vector|GetForwardVector (Pawn|GetControlRotation _returnvalue :!class /Script/Engine.Pawn)) "0.000000,0.000000,0.750000") 1e+03) true 0.0 "ECC_WorldDynamic" false (Utilities|Array|MakeArray _returnvalue 0) "ForOneFrame"))
  (if (Variables|Default|GetIsTargeting?)
    (Transformation|SetWorldLocation (Variables|/Script/Engine.Actor|GetRootComponent (stale _returnvalue_2)) (.ImpactPoint (Collision|BreakHitResult _outhit)) true false)
    (else
      (bind _returnvalue_2 (Game|SpawnActorfromClass "/Game/Blueprints/Lotus/BP_Root.BP_Root_C" (Math|Transform|MakeTransform (.Location (Collision|BreakHitResult _outhit)) (Math|Rotator|MakeRotfromZ (.Normal (Collision|BreakHitResult _outhit)))) "AlwaysSpawn" 0 0))
      (Variables|/Game/Blueprints/Lotus/BP_Root.BP_Root_C|SetRadius _returnvalue_2 1.5e+02)
      (Variables|Default|SetIsTargeting? true))))