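; BP_Root is a one-shot area spell effect in the Lotus folder that hits AI characters around it.
; On BeginPlay it sizes its sphere to Radius and queries that component for overlapping Character pawns.
; Each one implementing AIInterface receives a spell-hit message and a Skill1 mesh message scaled by frame delta time.
; The actor then destroys itself immediately, so it never ticks or tracks later overlaps.
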(event EventBeginPlay
  (Components|Sphere|SetSphereRadius (Variables|Default|GetSphere) (Variables|Default|GetRadius) true)
  (bind _outactors (Collision|ComponentOverlapActors (Variables|Default|GetSphere) (Transformation|GetWorldTransform (Variables|Default|GetSphere)) (Utilities|Array|MakeArray "ObjectTypeQuery3") "/Script/Engine.Character"))
  (for _array_element _outactors
    (if (Utilities|DoesObjectImplementInterface _array_element "/Game/AI/AIInterface.AIInterface_C")
      (Class|AIInterface|TriggerSpellHitAI(Message) _array_element 3.0)
      (Class|AIInterface|Skill1MeshCall(Message) _array_element (* (Utilities|Time|GetWorldDeltaSeconds) 2.0))))
  (Actor|DestroyActor))

(fn ConstructionScript)