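; BP_Interactable1 is an interactable that shows the player a sequence of dialogue lines.
; Overlapping its sphere shows a prompt widget for actors tagged Player, unless a cooldown is active.
; Each Talk call advances through the Dialogue array, displaying lines in a lazily created W_Message viewport widget.
; After the last line it removes the message, runs a short cooldown, then resets and restores the prompt if still overlapped.
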(event OnComponentBeginOverlap(Sphere)
  (params (OverlappedComponent :type Primitive%20Component%20Object%20Reference) (OtherActor :type Actor%20Object%20Reference) (OtherComp :type Primitive%20Component%20Object%20Reference) (OtherBodyIndex :type Integer) (bFromSweep :type Boolean) (SweepResult :type Hit%20Result%20Structure%20%28by%20ref%29))
  (if (and (Actor|ActorHasTag OtherActor "Player") (not (Variables|Default|GetCooldown)))
    (Variables|Default|SetOverlap true)
    (Rendering|SetVisibility (Variables|Default|GetWidget) true false)))

(event OnComponentEndOverlap(Sphere)
  (params (OverlappedComponent :type Primitive%20Component%20Object%20Reference) (OtherActor :type Actor%20Object%20Reference) (OtherComp :type Primitive%20Component%20Object%20Reference) (OtherBodyIndex :type Integer))
  (if (Actor|ActorHasTag OtherActor "Player")
    (Variables|Default|SetOverlap false)
    (Rendering|SetVisibility (Variables|Default|GetWidget) false false)))

(event EventBeginPlay
  (Rendering|SetVisibility (Variables|Default|GetWidget) false false))

(event EventTalk
  (bind _widget (Variables|Default|GetWidget))
  (Math|Integer|IncrementInt (Variables|Default|GetTalkIndex)
    (:%20%20
      (if (< (Variables|Default|GetTalkIndex) (Utilities|Array|Length (Variables|Default|GetDialogue)))
        (Variables|Default|GetUI
          (:then
            _)
          (:else
            (bind _returnvalue (UserInterface|CreateWidget "/Game/GAS/InteractEnv/W_Message.W_Message_C" (Game|GetPlayerController 0)))
            (bind _output_get (Variables|Default|SetUI _returnvalue))
            (UserInterface|Viewport|AddtoViewport _output_get 0)))
        (Rendering|Components|TextRender|SetText (Variables|/Game/GAS/InteractEnv/W_Message.W_Message_C|GetMessageBlock (Variables|Default|GetUI)) (Utilities|Text|ToText(String) (Utilities|Array|Get(acopy) (Variables|Default|GetDialogue) (Variables|Default|GetTalkIndex))))
        (else
          (Widget|RemovefromParent (Variables|Default|GetUI))
          (Rendering|SetVisibility (Variables|Default|GetWidget) false false)
          (Variables|Default|SetCooldown true)
          (Utilities|FlowControl|Delay 3.0)
          (Variables|Default|SetCooldown false)
          (Variables|Default|SetTalkIndex -1)
          (Variables|Default|SetUI 0)
          (if (Variables|Default|GetOverlap)
            (Rendering|SetVisibility _widget true false)
            (else
              (Rendering|SetVisibility _widget false false))))))))

(fn ConstructionScript)